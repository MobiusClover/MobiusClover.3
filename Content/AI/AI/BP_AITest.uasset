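; BP_AITest is an AI test Blueprint with a mesh and capsule that configures its collision when play begins.
; After the parent BeginPlay, the mesh becomes a query-and-physics PhysicsBody, and both components are set to block all channels.
; Exceptions then make the mesh ignore Pawn and Vehicle and the capsule ignore Visibility, so the capsule does not block visibility traces while the mesh still does.
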(event EventBeginPlay
  (|CallParentFunction)
  (Collision|SetCollisionEnabled (Variables|Character|GetMesh) "QueryAndPhysics")
  (Collision|SetCollisionObjectType (Variables|Character|GetMesh) "ECC_PhysicsBody")
  (Collision|SetCollisionResponsetoAllChannels (Variables|Character|GetMesh) "ECR_Block")
  (Collision|SetCollisionResponsetoChannel (Variables|Character|GetMesh) "ECC_Pawn" "ECR_Ignore")
  (Collision|SetCollisionResponsetoChannel (Variables|Character|GetMesh) "ECC_Vehicle" "ECR_Ignore")
  (Collision|SetCollisionResponsetoChannel (Variables|Default|GetCapsuleComponent) "ECC_Visibility" "ECR_Ignore"))

(fn ConstructionScript)